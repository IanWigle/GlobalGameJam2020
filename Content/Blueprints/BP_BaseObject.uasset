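; BP_BaseObject is a base object that can be picked up, carried and placed on a StatueStand.
; Pickup stops its fade, disables mesh physics and attaches it to the supplied component, detaching first when overlapping a stand.
; Drop detaches it and restores physics unless MInStand is set, then attaches it to the first overlapping stand's build area, keeping world transform.
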(event EventPickup
  (params (AttachTo :type Scene%20Component%20Object%20Reference))
  (if (> (Utilities|Array|Length (Collision|GetOverlappingActors "/Script/GlobalGameJam2020.StatueStand" :!class /Script/Engine.Actor)) 0)
    (Transformation|DetachFromActor "KeepRelative" "KeepRelative" "KeepRelative"))
  (Class|BaseObject|StopFade)
  (Variables|Default|Setm_BeingHeld true)
  (Physics|SetSimulatePhysics (Variables|Default|Getm_Mesh) false)
  (Transformation|AttachComponentToComponent (VehicleSound|GetRootComponent) AttachTo "None" "KeepWorld" "KeepWorld" "KeepWorld" false))

(event EventDrop
  (bind _overlappingactors (Collision|GetOverlappingActors "/Script/GlobalGameJam2020.StatueStand" :!class /Script/Engine.Actor))
  (Variables|Default|Setm_BeingHeld false)
  (if (Variables|Default|Getm_InStand)
    _
    (else
      (Physics|SetSimulatePhysics (Variables|Default|Getm_Mesh) true)))
  (Transformation|DetachFromActor "KeepWorld" "KeepWorld" "KeepWorld")
  (if (> (Utilities|Array|Length _overlappingactors) 0)
    (bind _asstatue_stand (Utilities|Casting|CastToStatueStand (Utilities|Array|Get(acopy) _overlappingactors)))
    (Transformation|AttachComponentToComponent (VehicleSound|GetRootComponent) (Variables|/Script/GlobalGameJam2020.StatueStand|Getm_BuildArea _asstatue_stand) "None" "KeepWorld" "KeepWorld" "KeepWorld" false)))

(fn ConstructionScript)