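; VR control panel actor that spins a referenced Statue left or right when a motion controller touches one of two trigger boxes.
; Overlaps by BP_MotionController set mutually exclusive direction flags and switch that side's indicator material from red to green, reverting on exit.
; Tick changes the statue's yaw by RotationSpeed scaled by delta seconds, adding for left and subtracting for right.
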(event OnComponentBeginOverlap(RightBox)
  (params (OverlappedComponent :type Primitive%20Component%20Object%20Reference) (OtherActor :type Actor%20Object%20Reference) (OtherComp :type Primitive%20Component%20Object%20Reference) (OtherBodyIndex :type Integer) (bFromSweep :type Boolean) (SweepResult :type Hit%20Result%20Structure%20%28by%20ref%29))
  (Utilities|Casting|CastToBP_MotionController OtherActor)
  (Variables|Default|SetIsMovingRight true)
  (Variables|Default|SetIsMovingLeft false)
  (Rendering|Material|SetMaterial (Variables|Stucture|GetRight) 0 "/Game/Materials/Green.Green"))

(event OnComponentEndOverlap(RightBox)
  (params (OverlappedComponent :type Primitive%20Component%20Object%20Reference) (OtherActor :type Actor%20Object%20Reference) (OtherComp :type Primitive%20Component%20Object%20Reference) (OtherBodyIndex :type Integer))
  (Utilities|Casting|CastToBP_MotionController OtherActor)
  (Variables|Default|SetIsMovingRight false)
  (Rendering|Material|SetMaterial (Variables|Stucture|GetRight) 0 "/Game/Materials/Red.Red"))

(event OnComponentBeginOverlap(LeftBox)
  (params (OverlappedComponent :type Primitive%20Component%20Object%20Reference) (OtherActor :type Actor%20Object%20Reference) (OtherComp :type Primitive%20Component%20Object%20Reference) (OtherBodyIndex :type Integer) (bFromSweep :type Boolean) (SweepResult :type Hit%20Result%20Structure%20%28by%20ref%29))
  (Utilities|Casting|CastToBP_MotionController OtherActor)
  (Variables|Default|SetIsMovingLeft true)
  (Variables|Default|SetIsMovingRight false)
  (Rendering|Material|SetMaterial (Variables|Stucture|GetLeft) 0 "/Game/Materials/Green.Green"))

(event OnComponentEndOverlap(LeftBox)
  (params (OverlappedComponent :type Primitive%20Component%20Object%20Reference) (OtherActor :type Actor%20Object%20Reference) (OtherComp :type Primitive%20Component%20Object%20Reference) (OtherBodyIndex :type Integer))
  (Utilities|Casting|CastToBP_MotionController OtherActor)
  (Variables|Default|SetIsMovingLeft false)
  (Rendering|Material|SetMaterial (Variables|Stucture|GetLeft) 0 "/Game/Materials/Red.Red"))

(event EventTick
  (params (DeltaSeconds :type Float%20%28single-precision%29))
  (bind _returnvalue (Utilities|Time|GetWorldDeltaSeconds))
  (bind _rotationspeed (Variables|Default|GetRotationSpeed))
  (bind _statue (Variables|Default|GetStatue))
  (bind _statue_2 (Variables|Default|GetStatue))
  (bind _returnvalue_2 (Transformation|GetActorRotation _statue))
  (bind _returnvalue_3 (Transformation|GetActorRotation _statue))
  (bind _returnvalue_4 (* _rotationspeed _returnvalue))
  (bind (_roll _pitch _yaw) (Math|Rotator|BreakRotator _returnvalue_2))
  (bind (_roll_2 _pitch_2 _yaw_2) (Math|Rotator|BreakRotator _returnvalue_3))
  (Utilities|IsValid (Variables|Default|GetStatue)
    (:Is%20Valid
      (if (Variables|Default|GetIsMovingLeft)
        (Transformation|SetActorRotation _statue_2 (Math|Rotator|MakeRotator _roll _pitch (+ _yaw _returnvalue_4)) true)
        (elif (Variables|Default|GetIsMovingRight)
          (Transformation|SetActorRotation _statue_2 (Math|Rotator|MakeRotator _roll_2 _pitch_2 (- _yaw_2 _returnvalue_4)) true))))))

(event EventBeginPlay
  (Rendering|Material|SetMaterial (Variables|Stucture|GetRight) 0 "/Game/Materials/Red.Red")
  (Rendering|Material|SetMaterial (Variables|Stucture|GetLeft) 0 "/Game/Materials/Red.Red"))

(fn ConstructionScript)